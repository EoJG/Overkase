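; BP_Test is a test Blueprint that triggers the interaction of an EO_Block it has overlapped.
; An actor overlap casts the other actor to EO_Block and stores it as the current Block, with nothing clearing it afterwards.
; The F key flips a boolean through a FlipFlop, and while it is true, Tick calls Interaction on the stored Block every frame without a validity check.
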(event `self.ReceiveActorBeginOverlap`
  (params (OtherActor :type "Actor Object Reference"))
  (bind _aseo_block (cast `EO_Block` OtherActor))
  (set `self.block` _aseo_block))

(event `self.ReceiveTick`
  (params (DeltaSeconds :type "Float (single-precision)"))
  (if (`self.b`)
    (`EO_Block.Interaction` (`self.block`))))

(event `Key|F`
  (params (Key :type "Key Structure"))
  (:`Pressed`
    (`/Engine/EditorBlueprintResources/StandardMacros.FlipFlop`
      (:`A`
        (set `self.b` true))
      (:`B`
        (set `self.b` false)))))

(fn `UserConstructionScript`)