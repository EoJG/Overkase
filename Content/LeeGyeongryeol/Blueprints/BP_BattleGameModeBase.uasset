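; Battle game mode that keeps a minutes-and-seconds countdown clock.
; Tick feeds a one-second Delay, so the clock steps down roughly once per second, rolling Seconds over into Minutes.
; The countdown holds at zero with no end-of-time action in this graph.
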(event `self.ReceiveTick`
  (params (DeltaSeconds :type "Float (single-precision)"))
  (`KismetSystemLibrary.Delay` 1.0)
  (if (== (`self.Seconds`) 0.0)
    (if (not (== (`self.Minutes`) 0))
      (set `self.Seconds` 59.0)
      (set `self.Minutes` (- (`self.Minutes`) 1)))
    (else
      (set `self.Seconds` (- (`self.Seconds`) 1.0)))))

(fn `UserConstructionScript`)